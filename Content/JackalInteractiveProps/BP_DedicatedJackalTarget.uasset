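; A task target prop dedicated to one JackalRobot, which finishes its task when that robot overlaps it while Reward is positive.
; On BeginPlay, it keeps a preassigned robot or picks a random Jackal from the level.
; A billboard text child actor shows the assigned Jackal's ID, or a warning when no robot is valid, in which case Reward is zeroed.
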(event `self.ReceiveBeginPlay`
  (`self.DedicatedRobot`
    (:`then`
      (`self.UpdateText`))
    (:`else`
      (`self.AssignToRandomJackal`))))

(event `self.ReceiveActorBeginOverlap`
  (params (OtherActor :type "Actor Object Reference"))
  (if (and (== OtherActor (`self.DedicatedRobot`)) (> (`self.Reward`) 0.0))
    (`self.FinishTask`)))

(event `UpdateText`
  (bind _asbp_billboard_text_render (cast `/Game/Core/Debug/BP_BillboardTextRender` (`ChildActorComponent.ChildActor` (`self.BP_BillboardTextRender`))))
  (bind _dedicatedrobot (`self.DedicatedRobot`)
    (:`then`
      (`KismetSystemLibrary.DelayUntilNextTick`)
      (`/Game/Core/Debug/BP_BillboardTextRender.SetText` _asbp_billboard_text_render (`KismetStringLibrary.Concat_StrStr` "Jackal" (`KismetStringLibrary.Conv_IntToString` (`JackalRobot.GetJackalId` _dedicatedrobot)))))
    (:`else`
      (`/Game/Core/Debug/BP_BillboardTextRender.SetText` _asbp_billboard_text_render "[No valid Jackal]")
      (set `self.Reward` 0.0))))

(fn `AssignToRandomJackal`
  (bind _outactors (`GameplayStatics.GetAllActorsOfClass` "/Script/Beryl.JackalRobot"))
  (bind _output_get (set `self.DedicatedRobot` (`KismetArrayLibrary.Array_Random` _outactors)))
  (set `self.IDJackal` (`JackalRobot.GetJackalId` _output_get))
  (`self.UpdateText`))

(fn `UserConstructionScript`
  (`parent.UserConstructionScript`))