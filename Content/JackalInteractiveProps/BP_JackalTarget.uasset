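; Jackal interactive prop target that completes its task when a JackalRobot overlaps it while its Reward is positive.
; Completion calls FinishPropTask, switches the billboard sprite to a checkmark and disables collision on its sphere.
; The overlap then clears the KeyName value in that robot's AI Blackboard.
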(event `self.ReceiveActorBeginOverlap`
  (params (OtherActor :type "Actor Object Reference"))
  (if (> (`self.Reward`) 0.0)
    (bind _asjackal_robot (cast `JackalRobot` OtherActor))
    (`self.FinishTask`)
    (`BlackboardComponent.ClearValue` (`AIBlueprintHelperLibrary.GetBlackboard` _asjackal_robot) (`self.Key Name`))))

(event `FinishTask`
  (`self.FinishPropTask`)
  (`BillboardComponent.SetSprite` (`self.Billboard`) "/Game/Core/StatusIcons/check-mark.check-mark")
  (`PrimitiveComponent.SetCollisionEnabled` (`self.Sphere1`) "NoCollision"))

(fn `UserConstructionScript`)