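; Pawn Blueprint for a Jackal robot that scans for targets, exchanges comms messages and shows its power and battery state.
; BeginPlay assigns body and wheel meshes, binds comms and battery events, then signals readiness a tick later.
; Sensor scans feed SpatialMemory, which sets the HaveTarget blackboard flag when JackalTarget positions exist.
; Messages appear on temporary debug billboards, while power and battery events recolor indicator spheres by swapping materials.
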(event `BroadcastPingMessage`
  ;[0 0.1838 0.2066 0.5] Message Debug
  (bind _returnvalue (`CommsMessage.CreateCommsMessage` self (`self.GetJackalId`) (`self.K2_GetActorLocation` self) -1 (`GameplayStatics.GetTimeSeconds`)))
  (`CommsComponent.BroadcastMessage` (`self.CommsComponent`) _returnvalue))

(event `OnMessageReceived_Event`
  (params (Message :type "CommsMessage Object Reference"))
  ;[0 0.1838 0.2066 0.5] Message Debug
  (`self.DisplayMessage` Message))

(event `DisplayMessage`
  (params (Message :type "CommsMessage Object Reference") (IsEmitter :type Boolean))
  ;[0 0.1838 0.2066 0.5] Message Debug
  (`/Engine/EditorBlueprintResources/StandardMacros.IsValid` (`self.CurrentMessageBillboard`)
    (:`Is Valid`
      (`ActorComponent.K2_DestroyComponent` (`self.CurrentMessageBillboard`)))
    (:`Is Not Valid`
      _))
  (bind _returnvalue (`AddComponent|NODE_AddChildActorComponent-1`))
  (bind _output_get (set `self.CurrentMessageBillboard` _returnvalue))
  (bind _asbp_billboard_text_render (cast `/Game/Core/Debug/BP_BillboardTextRender` (`ChildActorComponent.ChildActor` _output_get)))
  (`/Game/Core/Debug/BP_BillboardTextRender.SetText` _asbp_billboard_text_render (`KismetStringLibrary.Concat_StrStr` (`KismetMathLibrary.SelectString` " EMIT:" " RECEIVE:" IsEmitter) " \nJackal" (`KismetStringLibrary.Conv_IntToString` (`self.GetJackalId`)) " \nOutID=" (`KismetStringLibrary.Conv_IntToString` (`CommsMessage.SenderID` Message)) " \nDestID=" (`KismetStringLibrary.Conv_IntToString` (`CommsMessage.TargetReceiverID` Message)) " \nTime=" (`KismetTextLibrary.Conv_TextToString` (`KismetTextLibrary.Conv_DoubleToText` (`CommsMessage.Timestamp` Message) "HalfToEven" false true 1 324 1 1))))
  (`TextRenderComponent.SetWorldSize` (`TextRenderActor.TextRender` _asbp_billboard_text_render) 8.0)
  (`SceneComponent.K2_SetWorldLocation` (`self.CurrentMessageBillboard`) (+ (`SceneComponent.K2_GetComponentLocation` (`self.jackal-base`)) (0.0 0.0 100.0)) false false)
  (`KismetSystemLibrary.RetriggerableDelay` 7.0)
  (`ActorComponent.K2_DestroyComponent` (`self.CurrentMessageBillboard`)))

(event `OnMessageEmitted_Event`
  (params (Message :type "CommsMessage Object Reference"))
  ;[0 0.1838 0.2066 0.5] Message Debug
  (`self.DisplayMessage` Message true))

(event `self.Sensor.OnScanCompleted`
  (params (ScanResults :type "Array of Actor Object Reference"))
  (bind _spatialmemory (`self.SpatialMemory`))
  (`SpatialMemoryComponent.StoreDetectedActorsArray` _spatialmemory ScanResults)
  (bind _returnvalue (`SpatialMemoryComponent.GetAllPropsTypePos` _spatialmemory "JackalTarget"))
  (if (> (`BlueprintMapLibrary.Map_Length` _returnvalue) 0)
    (`BlackboardComponent.SetValueAsBool` (`AIBlueprintHelperLibrary.GetBlackboard` null) "HaveTarget" true)))

(event `self.ReceiveBeginPlay`
  (bind _commscomponent (`self.CommsComponent`))
  ;[0 0.2865 0.1311 0.722] BeginPlay
  (set `self.BodyMesh` (`self.jackal-base`))
  (set `self.WheelRearRight` (`self.jackal-wheel_rear_right`))
  (set `self.WheelRearLeft` (`self.jackal-wheel-rear_left`))
  (set `self.WheelFrontLeft` (`self.jackal-wheel-front_left`))
  (set `self.WheelFrontRight` (`self.jackal-wheel-front_right`))
  (set `CommsComponent.CommsArea` (`self.CommsCollision`) _commscomponent)
  (add `CommsComponent.OnMessageEmitted` _commscomponent (delegate `OnMessageEmitted_Event`))
  (add `CommsComponent.OnMessageReceived` _commscomponent (delegate `OnMessageReceived_Event`))
  (add `self.OnPowerChanged` (delegate `OnPowerChanged_Event`))
  (add `self.OnBatteryFull` (delegate `OnBatteryFull_Event`))
  (add `self.OnBatteryHigh` (delegate `OnBatteryHigh_Event`))
  (add `self.OnBatteryLow` (delegate `OnBatteryLow_Event`))
  (add `self.OnBatteryCritical` (delegate `OnBatteryCritical_Event`))
  (`KismetSystemLibrary.DelayUntilNextTick`)
  (`self.JackalReady`))

(event `OnBatteryFull_Event`
  ;[0 0.1838 0.2066 0.5] Battery state display
  (`self.SetBatteryIndicator` :!label _label))

(event `OnBatteryHigh_Event`
  ;[0 0.1838 0.2066 0.5] Battery state display
  (goto _label))

(event `OnBatteryLow_Event`
  ;[0 0.1838 0.2066 0.5] Battery state display
  (goto _label))

(event `OnBatteryCritical_Event`
  ;[0 0.1838 0.2066 0.5] Battery state display
  (goto _label))

(event `OnPowerChanged_Event` :!signature `self.OnPowerChanged`
  (params (bIsJackalOn :type Boolean))
  ;[0 0.1838 0.2066 0.5] Battery state display
  (if bIsJackalOn
    (`PrimitiveComponent.SetMaterial` (`self.SpherePower`) 0 "/Game/JackalRobot/jackal_icons/MI_hmi-indicator_blue.MI_hmi-indicator_blue")
    (`PrimitiveComponent.SetMaterial` (`self.SphereComms`) 0 "/Game/JackalRobot/jackal_icons/MI_hmi-indicator_green.MI_hmi-indicator_green")
    (`PrimitiveComponent.SetMaterial` (`self.SphereMotionStop`) 0 "/Game/JackalRobot/jackal_icons/MI_hmi-indicator_green.MI_hmi-indicator_green")
    (`PrimitiveComponent.SetMaterial` (`self.SphereWifi`) 0 "/Game/JackalRobot/jackal_icons/MI_hmi-indicator_green.MI_hmi-indicator_green")
    (`self.SetBatteryIndicator`)
    (else
      (`PrimitiveComponent.SetMaterial` (`self.SphereWifi`) 0 "/Game/JackalRobot/jackal_icons/MI_hmi-indicator_black.MI_hmi-indicator_black")
      (`PrimitiveComponent.SetMaterial` (`self.SphereComms`) 0 "/Game/JackalRobot/jackal_icons/MI_hmi-indicator_black.MI_hmi-indicator_black")
      (`PrimitiveComponent.SetMaterial` (`self.SphereMotionStop`) 0 "/Game/JackalRobot/jackal_icons/MI_hmi-indicator_black.MI_hmi-indicator_black")
      (`PrimitiveComponent.SetMaterial` (`self.SphereBattery`) 0 "/Game/JackalRobot/jackal_icons/MI_hmi-indicator_black.MI_hmi-indicator_black")
      (`PrimitiveComponent.SetMaterial` (`self.SpherePower`) 0 "/Game/JackalRobot/jackal_icons/MI_hmi-indicator_black.MI_hmi-indicator_black"))))

(event `SetBatteryIndicator`
  ;[0 0.1838 0.2066 0.5] Battery state display
  (switch `EBatteryState` (`self.BatteryState`)
    (:`BatteryFull`
      (`PrimitiveComponent.SetMaterial` (`self.SphereBattery`) 0 "/Game/JackalRobot/jackal_icons/MI_hmi-indicator_green.MI_hmi-indicator_green" :!label _label_2))
    (:`BatteryHigh`
      (goto _label_2))
    (:`BatteryLow`
      (`PrimitiveComponent.SetMaterial` (`self.SphereBattery`) 0 "/Game/JackalRobot/jackal_icons/MI_hmi-indicator_yellow.MI_hmi-indicator_yellow"))
    (:`BatteryCritical`
      (`PrimitiveComponent.SetMaterial` (`self.SphereBattery`) 0 "/Game/JackalRobot/jackal_icons/MI_hmi-indicator_red.MI_hmi-indicator_red"))
    (:`BatteryEmpty`
      (`PrimitiveComponent.SetMaterial` (`self.SphereBattery`) 0 "/Game/JackalRobot/jackal_icons/MI_hmi-indicator_black.MI_hmi-indicator_black"))))

(fn `UserConstructionScript`)